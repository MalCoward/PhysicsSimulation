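; Player controller that spawns level-specific Newton or Euler actors on key presses.
; N spawns the Newton actor only in LevelOne, while M spawns the Euler variant matching LevelOne or LevelTwo.
; Each press checks the current level name by string comparison and spawns a new half-scale actor at a fixed point above the origin.
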(event Input|KeyboardEvents|N
  (params (Key :type Key%20Structure :default "None"))
  (:Pressed
    (bind _returnvalue (Game|GetCurrentLevelName true))
    (if (Utilities|Enum|Equal(Enum) _returnvalue "LevelOne")
      (Game|SpawnActorfromClass "/Game/Blueprints/LevelOneNewton_BP.LevelOneNewton_BP_C" (Math|Transform|MakeTransform "0, 0,110.000000" "0, 0, 0" "0.500000,0.500000,0.500000") "Undefined" 0 0))))

(event Input|KeyboardEvents|M
  (params (Key :type Key%20Structure :default "None"))
  (:Pressed
    (bind _returnvalue (Game|GetCurrentLevelName true))
    (if (Utilities|Enum|Equal(Enum) _returnvalue "LevelOne")
      (Game|SpawnActorfromClass "/Game/Blueprints/LevelOneEuler_BP.LevelOneEuler_BP_C" (Math|Transform|MakeTransform "0, 0,110.000000" "0, 0, 0" "0.500000,0.500000,0.500000") "Undefined" 0 0)
      (else
        (bind _returnvalue_2 (Game|GetCurrentLevelName true))
        (if (Utilities|Enum|Equal(Enum) _returnvalue_2 "LevelTwo")
          (Game|SpawnActorfromClass "/Game/Blueprints/LevelTwoEuler_BP.LevelTwoEuler_BP_C" (Math|Transform|MakeTransform "0, 0,110.000000" "0, 0, 0" "0.500000,0.500000,0.500000") "Undefined" 0 0))))))

(fn ConstructionScript)